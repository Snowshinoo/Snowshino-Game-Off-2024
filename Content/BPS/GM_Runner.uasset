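; Runner game mode that manages a level's start, enemy-count goal and completion.
; BeginPlay caches the player and opens the start widget with UI-only input.
; Enemy decrements update the HUD and flag the goal at zero; CompleteLevel then stops the timer and shows final time.
; Leaderboard lookup is unfinished, reading BestTime without level matching while displaying zero; fail and clue handlers are stubs.
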(event EventBeginPlay
  (bind _ascbp_player (Utilities|Casting|CastToCBP_Player (Game|GetPlayerCharacter 0)))
  (Variables|Default|SetAs%20CBP%20Player _ascbp_player)
  (CallFunction|StartLevel))

(fn ConstructionScript)

(fn StartLevel
  (bind _aspc_player (Utilities|Casting|CastToPC_Player (Game|GetPlayerController 0)))
  (bind _output_get (Variables|Default|SetAs%20PC%20Player _aspc_player))
  (Variables|/Script/Engine.PlayerController|SetbShowMouseCursor _output_get true)
  (bind _returnvalue (UserInterface|CreateWidget "/Game/BPS/Widgets/WBP_StartLevel.WBP_StartLevel_C" _output_get))
  (bind _output_get_2 (Variables|Default|SetStartLevelWidget _returnvalue))
  (UserInterface|Viewport|AddtoViewport _output_get_2 0)
  (Input|SetInputModeUIOnly (Variables|Default|GetAs%20PC%20Player) _output_get_2 "DoNotLock" false))

(fn CompleteLevel
  (bind _returnvalue (Game|GetPlayerController 0))
  (if (== (Variables|goal|GetLevelEnemyCount) 0)
    (Utilities|FlowControl|Sequence
      (:then_0
        (bind _ascbp_player (Utilities|Casting|CastToCBP_Player (Game|GetPlayerCharacter 0)))
        (Variables|/Game/BPS/Widgets/WBP_Timer.WBP_Timer_C|SetTimerEnabled? (Variables|/Game/BPS/Widgets/WBP_Hud.WBP_Hud_C|GetWBP_Timer (Variables|/Game/BPS/CBP_Player.CBP_Player_C|GetHudWidget _ascbp_player)) false)
        (bind _returnvalue_2 (UserInterface|CreateWidget "/Game/BPS/Widgets/WBP_LevelComplete.WBP_LevelComplete_C" (Game|GetPlayerController 0)))
        (UserInterface|Viewport|AddtoViewport _returnvalue_2 0)
        (Default|FinalTime _returnvalue_2 (Variables|/Game/BPS/Widgets/WBP_Timer.WBP_Timer_C|GetElapsedTime (Variables|/Game/BPS/Widgets/WBP_Hud.WBP_Hud_C|GetWBP_Timer (Variables|/Game/BPS/CBP_Player.CBP_Player_C|GetHudWidget _ascbp_player))))
        (CallFunction|SetLeaderboardData)
        (Default|BestTimeSet _returnvalue_2 0.0))
      (:then_1
        (AI|Navigation|StopMovement _returnvalue)
        (Input|SetInputModeUIOnly _returnvalue 0 "DoNotLock" true)
        (Variables|/Script/Engine.PlayerController|SetbShowMouseCursor _returnvalue true)))))

(fn FailLevel)

(fn SetLeaderboardData
  (bind _returnvalue (Game|GetCurrentLevelName true))
  (bind _outrownames (DataTable|GetDataTableRowNames "/Game/BPS/Goal/DT_LevelName.DT_LevelName"))
  (for _array_element _outrownames
    (bind _returnvalue_2 (Utilities|GetDataTableRow "/Game/BPS/Goal/DT_LevelName.DT_LevelName" _array_element)
      (:then
        (Variables|Default|SetBest%20Time (.BestTime (Utilities|Struct|BreakSt_Leaderboard _returnvalue_2)))))))

(fn ClueFoundinlevel
  (params (Cluename :type String) (ClueFound? :type Boolean))
  (Game|GetCurrentLevelName true))

(fn SetEnemyCount
  (params (EnemyCountStart :type Integer))
  (bind _output_get (Variables|goal|SetLevelEnemyCount EnemyCountStart)))

(fn LowerEnemyCount
  (bind _result (Math|Integer|DecrementInt (Variables|goal|GetLevelEnemyCount))
    (:%20%20
      (bind _output_get (Variables|goal|SetLevelEnemyCount _result))
      (if (<= _output_get 0)
        (Variables|Default|SetLevelgoalComplete? true))
      (Default|UpdateEnemyCount (Variables|/Game/BPS/Widgets/WBP_Hud.WBP_Hud_C|GetWBP_EnemyCount (Variables|/Game/BPS/CBP_Player.CBP_Player_C|GetHudWidget (Variables|Default|GetAs%20CBP%20Player))) _output_get))))