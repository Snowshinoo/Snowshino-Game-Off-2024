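; BP_EnemyBullet is an enemy projectile that damages the player on overlap.
; Any overlap on the Bullet component spawns a Niagara burst at the other actor's location and destroys the projectile.
; A separate DamageSphere overlap applies damage only to CBP_Player, then destroys the projectile.
; Both handlers print debug strings, and no movement logic appears in the graphs.
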(event OnComponentBeginOverlap(Bullet)
  (params (OverlappedComponent :type Primitive%20Component%20Object%20Reference) (OtherActor :type Actor%20Object%20Reference) (OtherComp :type Primitive%20Component%20Object%20Reference) (OtherBodyIndex :type Integer) (bFromSweep :type Boolean) (SweepResult :type Hit%20Result%20Structure%20%28by%20ref%29))
  (Development|PrintString "IMPACT" true true "(R=0.000000,G=1.000000,B=0.281196,A=1.000000)")
  (Niagara|SpawnSystematLocation "/Game/Niagra/NS_BulletBurst.NS_BulletBurst" (Transformation|GetActorLocation OtherActor))
  (Actor|DestroyActor))

(event OnComponentBeginOverlap(DamageSphere)
  (params (OverlappedComponent :type Primitive%20Component%20Object%20Reference) (OtherActor :type Actor%20Object%20Reference) (OtherComp :type Primitive%20Component%20Object%20Reference) (OtherBodyIndex :type Integer) (bFromSweep :type Boolean) (SweepResult :type Hit%20Result%20Structure%20%28by%20ref%29))
  (bind _ascbp_player (Utilities|Casting|CastToCBP_Player OtherActor))
  (bind _returnvalue (Game|Damage|ApplyDamage _ascbp_player 1.0 0 0))
  (Development|PrintString (Utilities|String|ToString(Float) _returnvalue))
  (Actor|DestroyActor))

(event EventBeginPlay)

(event Collision|EventActorBeginOverlap
  (params (OtherActor :type Actor%20Object%20Reference)))

(event EventTick
  (params (DeltaSeconds :type Float%20%28single-precision%29)))

(fn ConstructionScript)